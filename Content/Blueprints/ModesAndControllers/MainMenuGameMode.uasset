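; Main menu game mode Blueprint with a LoadGame function for restoring saved player progress.
; LoadGame creates a fresh BallerSaveGame to get the default slot name (PlayerName) and user index (Slot), then loads that save.
; If the cast to BallerSaveGame succeeds, it copies Score, Level and Lives onto the player's BP_BallPawn.
; The LoadGame call in the event graph is unconnected, and BeginPlay and Tick are empty.
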(fn `Load game`
  (bind _asbp_ball_pawn (cast `/Game/Blueprints/Pawn/BP_BallPawn` (`GameplayStatics.GetPlayerPawn` 0) :!pure true))
  (bind _returnvalue (`GameplayStatics.CreateSaveGameObject` "/Game/Blueprints/ModesAndControllers/BallerSaveGame.BallerSaveGame_C"))
  (bind _returnvalue_2 (`GameplayStatics.LoadGameFromSlot` (`/Game/Blueprints/ModesAndControllers/BallerSaveGame.PlayerName` _returnvalue) (`/Game/Blueprints/ModesAndControllers/BallerSaveGame.Slot` _returnvalue)))
  (bind _asballer_save_game (cast `/Game/Blueprints/ModesAndControllers/BallerSaveGame` _returnvalue_2))
  (set `/Game/Blueprints/Pawn/BP_BallPawn.Score` (`/Game/Blueprints/ModesAndControllers/BallerSaveGame.Score` _asballer_save_game) _asbp_ball_pawn)
  (set `/Game/Blueprints/Pawn/BP_BallPawn.Level` (`/Game/Blueprints/ModesAndControllers/BallerSaveGame.Level` _asballer_save_game) _asbp_ball_pawn)
  (set `/Game/Blueprints/Pawn/BP_BallPawn.Lives` (`/Game/Blueprints/ModesAndControllers/BallerSaveGame.Lives` _asballer_save_game) _asbp_ball_pawn))

(fn `UserConstructionScript`)