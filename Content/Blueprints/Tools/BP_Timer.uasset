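; BP_Timer is a countdown timer actor that shows a Timer widget on screen and flags when time runs out.
; BeginPlay creates the widget, waits for the initial Countdown value in seconds, then sets OutOfTime.
; Separately, Tick uses a one-second Delay as a throttle to decrement Countdown, clamped between zero and sixty.
; The flag relies on its own delay rather than on Countdown reaching zero.
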(event `self.ReceiveBeginPlay`
  (bind _returnvalue (`|CreateWidget` "/Game/Blueprints/UI/Timer.Timer_C"))
  (`UserWidget.AddToViewport` _returnvalue 0)
  (`KismetSystemLibrary.Delay` (`KismetMathLibrary.Conv_IntToDouble` (stale `self.ReceiveTick` _output_get)))
  (set `self.OutOfTime` true))

(event `self.ReceiveTick`
  (params (DeltaSeconds :type "Float (single-precision)"))
  (`KismetSystemLibrary.Delay` 1.0)
  (bind _output_get (set `self.Countdown` (`KismetMathLibrary.Clamp` (- (`self.Countdown`) 1) 0 60))))

(fn `UserConstructionScript`)