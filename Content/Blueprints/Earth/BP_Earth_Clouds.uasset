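; BP_Earth_Clouds is an Earth actor that orients its Earth component to match the current UTC time of day.
; On BeginPlay it converts the UTC clock to a fraction of the day and maps that to a negative full-turn yaw, with a fixed roll tilt.
; The rotation is set only once, with no update afterward, and the construction script just calls its parent.
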(event `self.ReceiveBeginPlay`
  (bind _returnvalue (`KismetMathLibrary.UtcNow`))
  (`SceneComponent.K2_SetRelativeRotation` (`self.Earth`) (`KismetMathLibrary.MakeRotator` -60.0 0.0 (* (/ (+ (* (`KismetMathLibrary.GetHour` _returnvalue) 3600) (* (`KismetMathLibrary.GetMinute` _returnvalue) 60) (`KismetMathLibrary.GetSecond` _returnvalue)) 86399) -360.0)) false false))

(fn `UserConstructionScript`
  (`parent.UserConstructionScript`))