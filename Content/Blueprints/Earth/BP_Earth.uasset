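; BP_Earth is an Earth actor that orients its globe to match the current UTC time of day.
; It converts UTC hours, minutes and seconds into a day fraction, then into a negative yaw with a fixed offset, alongside a constant roll tilt.
; The same calculation and debug print run in the Construction Script and on BeginPlay, with no update afterwards.
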(event `self.ReceiveBeginPlay`
  (bind _returnvalue (`KismetMathLibrary.UtcNow`))
  (bind _returnvalue_2 (* (/ (+ (* (`KismetMathLibrary.GetHour` _returnvalue) 3600) (* (`KismetMathLibrary.GetMinute` _returnvalue) 60) (`KismetMathLibrary.GetSecond` _returnvalue)) 86399) -360.0))
  (`KismetSystemLibrary.PrintString` (`KismetStringLibrary.Conv_DoubleToString` _returnvalue_2))
  (`SceneComponent.K2_SetRelativeRotation` (`self.Earth`) (`KismetMathLibrary.MakeRotator` -23.0 0.0 (- _returnvalue_2 172.0)) false false))

(fn `UserConstructionScript`
  (bind _returnvalue (`KismetMathLibrary.UtcNow`))
  (bind _returnvalue_2 (* (/ (+ (* (`KismetMathLibrary.GetHour` _returnvalue) 3600) (* (`KismetMathLibrary.GetMinute` _returnvalue) 60) (`KismetMathLibrary.GetSecond` _returnvalue)) 86399) -360.0))
  (`KismetSystemLibrary.PrintString` (`KismetStringLibrary.Conv_DoubleToString` _returnvalue_2))
  (`SceneComponent.K2_SetRelativeRotation` (`self.Earth`) (`KismetMathLibrary.MakeRotator` -23.0 0.0 (- _returnvalue_2 172.0)) false false))