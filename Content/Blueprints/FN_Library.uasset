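; Function library for the ball game, covering buoyancy, save loading, death and ragdolling.
; Bouyancy line-traces down and pushes the component along the hit normal, weakening with distance, and sets damping.
; LoadGame copies saved score, level and lives onto BP_BallPawn.
; Death decrements lives, saves them with level and the previously saved score, then reopens the current level, while Ragdoll enables physics on the pawn's Cat.
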(fn `Bouyancy`
  (params (Float :type "PrimitiveComponent Object Reference") (`Float Height` :type "Float (double-precision)") (ObjectType :type "EObjectTypeQuery Enum" :default "ObjectTypeQuery1") (ForceStrength :type "Float (double-precision)"))
  (returns (IsFloating :type Boolean))
  (locals (NewLocalVar_0 :type "/Game/Blueprints/Pawn/BP_CatAnim Object Reference"))
  (bind _returnvalue (`SceneComponent.K2_GetComponentLocation` Float))
  (bind (_returnvalue_x _returnvalue_y _returnvalue_z) (`KismetMathLibrary.BreakVector` (`SceneComponent.K2_GetComponentScale` Float)))
  (bind _float (`local.Float`))
  (bind _float_2 (`local.Float`))
  (bind (_outhit _returnvalue_2) (`KismetSystemLibrary.LineTraceSingleForObjects` null _returnvalue (- _returnvalue (`KismetMathLibrary.MakeVector` 0.0 0.0 (+ (/ (+ _returnvalue_x _returnvalue_y _returnvalue_z) 3.0) `Float Height`))) (`|MakeArray` ObjectType)))
  (if _returnvalue_2
    (bind (_bblockinghit _binitialoverlap _time _distance _location _impactpoint _normal _impactnormal) (`GameplayStatics.BreakHitResult` _outhit))
    (`PrimitiveComponent.AddForce` _float (* _impactnormal (`KismetMathLibrary.Lerp` (* (`PrimitiveComponent.GetMass` _float_2) (`local.ForceStrength`)) 0.0 (/ (`KismetMathLibrary.VSize` (- _location (`SceneComponent.K2_GetComponentLocation` _float_2))) (`local.Float Height`)))) "None" false)
    (`PrimitiveComponent.AddForce` _float (* _impactnormal (`KismetMathLibrary.Lerp` (* (`PrimitiveComponent.GetMass` _float_2) (`local.ForceStrength`)) 0.0 (/ (`KismetMathLibrary.VSize` (- _location (`SceneComponent.K2_GetComponentLocation` _float_2))) (`local.Float Height`)))) "None" false)
    (`PrimitiveComponent.SetAngularDamping` _float 1.0)
    (`PrimitiveComponent.SetLinearDamping` _float 1.0)
    (return true)))

(fn `Death`
  (params (Object :type "Object Object Reference"))
  (bind _asbp_ball_pawn (cast `/Game/Blueprints/Pawn/BP_BallPawn` (`GameplayStatics.GetPlayerPawn` null) :!pure true))
  (bind _asbp_ball_pawn_2 (cast `/Game/Blueprints/Pawn/BP_BallPawn` Object))
  (set `/Game/Blueprints/Pawn/BP_BallPawn.Lives` (- (`/Game/Blueprints/Pawn/BP_BallPawn.Lives` _asbp_ball_pawn_2) 1) _asbp_ball_pawn_2)
  (bind _returnvalue (`GameplayStatics.CreateSaveGameObject` "/Game/Blueprints/ModesAndControllers/BallerSaveGame.BallerSaveGame_C"))
  (bind _playername (`/Game/Blueprints/ModesAndControllers/BallerSaveGame.PlayerName` _returnvalue))
  (bind _slot (`/Game/Blueprints/ModesAndControllers/BallerSaveGame.Slot` _returnvalue))
  (bind _returnvalue_2 (`GameplayStatics.LoadGameFromSlot` _playername _slot))
  (bind _asballer_save_game (cast `/Game/Blueprints/ModesAndControllers/BallerSaveGame` _returnvalue_2))
  (set `/Game/Blueprints/ModesAndControllers/BallerSaveGame.Score` (`/Game/Blueprints/ModesAndControllers/BallerSaveGame.Score` _asballer_save_game) _returnvalue)
  (set `/Game/Blueprints/ModesAndControllers/BallerSaveGame.Level` (`/Game/Blueprints/Pawn/BP_BallPawn.Level` _asbp_ball_pawn) _returnvalue)
  (set `/Game/Blueprints/ModesAndControllers/BallerSaveGame.Lives` (`/Game/Blueprints/Pawn/BP_BallPawn.Lives` _asbp_ball_pawn) _returnvalue)
  (`GameplayStatics.SaveGameToSlot` _returnvalue _playername _slot)
  (bind _returnvalue_3 (`GameplayStatics.GetCurrentLevelName` null))
  (`GameplayStatics.OpenLevel` null (`KismetStringLibrary.Conv_StringToName` _returnvalue_3)))

(fn `LoadGame`
  (bind _asbp_ball_pawn (cast `/Game/Blueprints/Pawn/BP_BallPawn` (`GameplayStatics.GetPlayerPawn` null) :!pure true))
  (bind _returnvalue (`GameplayStatics.CreateSaveGameObject` "/Game/Blueprints/ModesAndControllers/BallerSaveGame.BallerSaveGame_C"))
  (bind _returnvalue_2 (`GameplayStatics.LoadGameFromSlot` (`/Game/Blueprints/ModesAndControllers/BallerSaveGame.PlayerName` _returnvalue) (`/Game/Blueprints/ModesAndControllers/BallerSaveGame.Slot` _returnvalue)))
  (bind _asballer_save_game (cast `/Game/Blueprints/ModesAndControllers/BallerSaveGame` _returnvalue_2))
  (set `/Game/Blueprints/Pawn/BP_BallPawn.Score` (`/Game/Blueprints/ModesAndControllers/BallerSaveGame.Score` _asballer_save_game) _asbp_ball_pawn)
  (set `/Game/Blueprints/Pawn/BP_BallPawn.Level` (`/Game/Blueprints/ModesAndControllers/BallerSaveGame.Level` _asballer_save_game) _asbp_ball_pawn)
  (set `/Game/Blueprints/Pawn/BP_BallPawn.Lives` (`/Game/Blueprints/ModesAndControllers/BallerSaveGame.Lives` _asballer_save_game) _asbp_ball_pawn))

(fn `Ragdoll`
  (params (NewParam :type "Object Object Reference"))
  (bind _asbp_ball_pawn (cast `/Game/Blueprints/Pawn/BP_BallPawn` NewParam))
  (`PrimitiveComponent.SetSimulatePhysics` (`/Game/Blueprints/Pawn/BP_BallPawn.Cat` _asbp_ball_pawn) true))