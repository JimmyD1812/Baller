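; MainMenuPawn is a pawn with a ball mesh that holds helper functions for level loading and jump positioning.
; NextLevel opens the level whose name joins LevelName and the Level value.
; JumpAngle returns a point just below BallMesh's world location, shifted horizontally against player 0's pawn velocity by a small factor.
; The construction script is empty, and the file has no event logic that calls either function.
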(fn `JumpAngle`
  (returns (X :type "Float (double-precision)") (Y :type "Float (double-precision)") (Z :type "Float (double-precision)"))
  (bind (_returnvalue_x _returnvalue_y _returnvalue_z) (`KismetMathLibrary.BreakVector` (`SceneComponent.K2_GetComponentLocation` (`self.BallMesh`))))
  (bind (_returnvalue_x_2 _returnvalue_y_2) (`KismetMathLibrary.BreakVector` (`self.GetVelocity` (`GameplayStatics.GetPlayerPawn` 0))))
  (return (- _returnvalue_x (* _returnvalue_x_2 0.005)) (- _returnvalue_y (* _returnvalue_y_2 0.005)) (- _returnvalue_z 10.0)))

(fn `NextLevel`
  (`GameplayStatics.OpenLevel` (`KismetStringLibrary.Conv_StringToName` (`KismetStringLibrary.Concat_StrStr` (`self.Level Name`) (`KismetStringLibrary.Conv_IntToString` (`self.Level`))))))

(fn `UserConstructionScript`)