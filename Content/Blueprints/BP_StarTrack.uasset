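; BP_StarTrack lays out copies of a chosen Blueprint, presumably stars going by the asset name, along a spline track.
; The construction script divides the TrackSpline length by Spacing and adds a Child Actor Component at each interval, starting at the spline's start.
; Each component sits at the spline's local-space location for that distance, with BPToSpawn as its child class; rotation does not follow the spline.
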(fn `UserConstructionScript`
  (for _index (range (+ (`KismetMathLibrary.FFloor` (/ (`SplineComponent.GetSplineLength` (`self.TrackSpline`)) (`self.Spacing`))) 1))
    (bind _returnvalue (`AddComponent|NODE_AddChildActorComponent-3` :`RelativeTransform` (`KismetMathLibrary.MakeTransform` (`SplineComponent.GetLocationAtDistanceAlongSpline` (`self.TrackSpline`) (* _index (`self.Spacing`)) "Local"))))
    (`ChildActorComponent.SetChildActorClass` _returnvalue (`self.BP to Spawn`))))