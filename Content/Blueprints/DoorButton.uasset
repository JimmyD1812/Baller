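; Door button that sets a DoorOpen flag while a BP_BallPawn overlaps its sphere collision and clears it when the pawn leaves.
; A timeline plays on entry and reverses on exit, lerping the button mesh down and back up with a fixed squashed Z scale.
; A DoOnce in the timeline update plays one click sound per movement, resetting when the timeline finishes.
; The file only sets the flag and moves no door itself.
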(event `self.SphereCollision.OnComponentBeginOverlap`
  (params (OverlappedComponent :type "PrimitiveComponent Object Reference") (OtherActor :type "Actor Object Reference") (OtherComp :type "PrimitiveComponent Object Reference") (OtherBodyIndex :type Integer) (bFromSweep :type Boolean) (SweepResult :type "HitResult Structure (by ref)"))
  (cast `/Game/Blueprints/Pawn/BP_BallPawn` OtherActor)
  (set `self.DoorOpen` true)
  (bind (_direction _buttonmovement) (`Timeline|Timeline_0` :!label _label)
    (:`Update`
      (`SceneComponent.K2_SetRelativeTransform` (`self.Button`) (`KismetMathLibrary.MakeTransform` (`KismetMathLibrary.MakeVector` 0.0 0.0 (`KismetMathLibrary.Lerp` 0.0 -10.0 _buttonmovement)) (struct) (1.0 1.0 0.75)) false false)
      (`/Engine/EditorBlueprintResources/StandardMacros.DoOnce` false :!label _label_2
        (:`Completed`
          (`GameplayStatics.PlaySound2D` "/Game/Interface_And_Item_Sounds/Cues/Futuristic_Click_07_Cue.Futuristic_Click_07_Cue" 1.0 1.0 0.0 null null))))
    (:`Finished`
      (goto _label_2 :!via `Reset`))))

(event `self.SphereCollision.OnComponentEndOverlap`
  (params (OverlappedComponent :type "PrimitiveComponent Object Reference") (OtherActor :type "Actor Object Reference") (OtherComp :type "PrimitiveComponent Object Reference") (OtherBodyIndex :type Integer))
  (cast `/Game/Blueprints/Pawn/BP_BallPawn` OtherActor)
  (set `self.DoorOpen` false)
  (goto _label :!via `Reverse`))

(fn `UserConstructionScript`)