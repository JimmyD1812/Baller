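; Elevator floor actor that raises its static mesh once a DoorButton reports its door open, then destroys itself.
; Tick looks up a DoorButton actor by class until the reference is valid, then polls its DoorOpen flag.
; When the flag is set, a timeline lerps the mesh's relative height upward.
; A delay chained to the timeline's update, rather than its finish, triggers the destruction.
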(event `self.ReceiveTick`
  (params (DeltaSeconds :type "Float (single-precision)"))
  (`/Engine/EditorBlueprintResources/StandardMacros.IsValid` (`self.ButtonRef`)
    (:`Is Valid`
      (if (`/Game/Blueprints/DoorButton.DoorOpen` (`self.ButtonRef`))
        (bind (_direction _newtrack_0) (`Timeline|Timeline_0`)
          (:`Update`
            (`SceneComponent.K2_SetRelativeLocation` (`self.StaticMesh`) (`KismetMathLibrary.MakeVector` 0.0 0.0 (`KismetMathLibrary.Lerp` 0.0 300.0 _newtrack_0)) false false)
            (`KismetSystemLibrary.Delay` 2.0)
            (`self.K2_DestroyActor`)))))
    (:`Is Not Valid`
      (bind _returnvalue (`GameplayStatics.GetActorOfClass` "/Game/Blueprints/DoorButton.DoorButton_C"))
      (set `self.ButtonRef` _returnvalue))))

(fn `UserConstructionScript`)