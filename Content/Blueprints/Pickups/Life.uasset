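; Life pickup actor that adds one to a BallPawn's Lives when the pawn overlaps its sphere.
; Pickup plays a coin sound, spawns particles, hides the mesh and shows a PointsPopUp widget set to 1, then destroys the actor after a short delay.
; The sphere stays active during that delay, and the Spin and Bounce timelines for the mesh exist but are never started.
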(event `self.ReceiveBeginPlay`
  (bind _widget (`self.Widget`))
  (`SceneComponent.SetVisibility` _widget false false)
  (bind _aspoints_pop_up (cast `/Game/Blueprints/UI/PointsPopUp` (`WidgetComponent.GetWidget` _widget)))
  (set `/Game/Blueprints/UI/PointsPopUp.ScoreValue` 1 _aspoints_pop_up))

(event `self.Sphere.OnComponentBeginOverlap`
  (params (OverlappedComponent :type "PrimitiveComponent Object Reference") (OtherActor :type "Actor Object Reference") (OtherComp :type "PrimitiveComponent Object Reference") (OtherBodyIndex :type Integer) (bFromSweep :type Boolean) (SweepResult :type "HitResult Structure (by ref)"))
  ;[1 1 1] Increment Score
  (bind _asball_pawn (cast `/Game/Blueprints/Pawn/BallPawn` OtherActor))
  (set `/Game/Blueprints/Pawn/BallPawn.Lives` (+ (`/Game/Blueprints/Pawn/BallPawn.Lives` _asball_pawn) 1) _asball_pawn)
  (`GameplayStatics.PlaySound2D` "/Game/Interface_And_Item_Sounds/WAV/Coins_08.Coins_08" 1.0 1.0 0.0 null null)
  (`GameplayStatics.SpawnEmitterAtLocation` (`self.OnPickupParticles`) (`self.K2_GetActorLocation`))
  (`SceneComponent.SetVisibility` (`self.StaticMesh`) false false)
  (`SceneComponent.SetVisibility` (`self.Widget`) true false)
  (`KismetSystemLibrary.Delay` 0.75)
  (`self.K2_DestroyActor`))

(fn `UserConstructionScript`)