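; GameWin is a level-completion pickup that advances the ball player to the level named FinalLevel.
; When a BallPawn overlaps its sphere, it increments that pawn's Level and destroys itself.
; It then saves the player's score, level and lives to a new BallerSaveGame slot and opens FinalLevel.
; Spin and Bounce timeline logic for animating the mesh is present but never runs.
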(event `self.Sphere.OnComponentBeginOverlap`
  (params (OverlappedComponent :type "PrimitiveComponent Object Reference") (OtherActor :type "Actor Object Reference") (OtherComp :type "PrimitiveComponent Object Reference") (OtherBodyIndex :type Integer) (bFromSweep :type Boolean) (SweepResult :type "HitResult Structure (by ref)"))
  (bind _asball_pawn (cast `/Game/Blueprints/Pawn/BallPawn` (`GameplayStatics.GetPlayerPawn` 0) :!pure true))
  ;[1 1 1] Increment Level
  (bind _asball_pawn_2 (cast `/Game/Blueprints/Pawn/BallPawn` OtherActor))
  (set `/Game/Blueprints/Pawn/BallPawn.Level` (+ (`/Game/Blueprints/Pawn/BallPawn.Level` _asball_pawn_2) 1) _asball_pawn_2)
  (`self.K2_DestroyActor`)
  (bind _returnvalue (`GameplayStatics.CreateSaveGameObject` "/Game/Blueprints/BallerSaveGame.BallerSaveGame_C"))
  (set `/Game/Blueprints/BallerSaveGame.Score` (`/Game/Blueprints/Pawn/BallPawn.Score` _asball_pawn) _returnvalue)
  (set `/Game/Blueprints/BallerSaveGame.Level` (`/Game/Blueprints/Pawn/BallPawn.Level` _asball_pawn) _returnvalue)
  (set `/Game/Blueprints/BallerSaveGame.Lives` (`/Game/Blueprints/Pawn/BallPawn.Lives` _asball_pawn) _returnvalue)
  (`GameplayStatics.SaveGameToSlot` _returnvalue (`/Game/Blueprints/BallerSaveGame.PlayerName` _returnvalue) (`/Game/Blueprints/BallerSaveGame.Slot` _returnvalue))
  (`GameplayStatics.OpenLevel` "FinalLevel"))

(fn `UserConstructionScript`)