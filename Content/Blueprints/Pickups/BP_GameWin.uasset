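; BP_GameWin is a pickup that sends the player to FinalLevel when a BP_BallPawn overlaps its sphere.
; On overlap it increments the pawn's Level, destroys itself, saves the player pawn's Score, Level and Lives to a new BallerSaveGame, then opens the level.
; The save slot comes from that new object's own PlayerName and Slot values.
; Spin and Bounce mesh timelines exist but are never run.
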(event `self.Sphere.OnComponentBeginOverlap`
  (params (OverlappedComponent :type "PrimitiveComponent Object Reference") (OtherActor :type "Actor Object Reference") (OtherComp :type "PrimitiveComponent Object Reference") (OtherBodyIndex :type Integer) (bFromSweep :type Boolean) (SweepResult :type "HitResult Structure (by ref)"))
  (bind _asbp_ball_pawn (cast `/Game/Blueprints/Pawn/BP_BallPawn` (`GameplayStatics.GetPlayerPawn` 0) :!pure true))
  ;[1 1 1] Increment Level
  (bind _asbp_ball_pawn_2 (cast `/Game/Blueprints/Pawn/BP_BallPawn` OtherActor))
  (set `/Game/Blueprints/Pawn/BP_BallPawn.Level` (+ (`/Game/Blueprints/Pawn/BP_BallPawn.Level` _asbp_ball_pawn_2) 1) _asbp_ball_pawn_2)
  (`self.K2_DestroyActor`)
  (bind _returnvalue (`GameplayStatics.CreateSaveGameObject` "/Game/Blueprints/ModesAndControllers/BallerSaveGame.BallerSaveGame_C"))
  (set `/Game/Blueprints/ModesAndControllers/BallerSaveGame.Score` (`/Game/Blueprints/Pawn/BP_BallPawn.Score` _asbp_ball_pawn) _returnvalue)
  (set `/Game/Blueprints/ModesAndControllers/BallerSaveGame.Level` (`/Game/Blueprints/Pawn/BP_BallPawn.Level` _asbp_ball_pawn) _returnvalue)
  (set `/Game/Blueprints/ModesAndControllers/BallerSaveGame.Lives` (`/Game/Blueprints/Pawn/BP_BallPawn.Lives` _asbp_ball_pawn) _returnvalue)
  (`GameplayStatics.SaveGameToSlot` _returnvalue (`/Game/Blueprints/ModesAndControllers/BallerSaveGame.PlayerName` _returnvalue) (`/Game/Blueprints/ModesAndControllers/BallerSaveGame.Slot` _returnvalue))
  (`GameplayStatics.OpenLevel` "FinalLevel"))

(fn `UserConstructionScript`)