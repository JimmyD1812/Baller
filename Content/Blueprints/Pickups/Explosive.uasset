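; Explosive bomb pickup that blasts the player's BallPawn when it enters the sphere trigger.
; BeginPlay plays a spark sound, hides the widget and presets its PointsPopUp score, though the widget is never shown here.
; On overlap it plays explosion effects, applies a velocity-change radial impulse from below the bomb to launch the ball, then destroys itself.
; Spin and bounce timeline logic for the mesh exists but never runs.
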(event `self.ReceiveBeginPlay`
  (bind _widget (`self.Widget`))
  (`GameplayStatics.PlaySoundAtLocation` "/Game/StarterContent/Audio/Fire_Sparks01_Cue.Fire_Sparks01_Cue" (`self.K2_GetActorLocation`) (struct) 1.0 1.0 0.0 null null null null)
  (`SceneComponent.SetVisibility` _widget false false)
  (bind _aspoints_pop_up (cast `/Game/Blueprints/UI/PointsPopUp` (`WidgetComponent.GetWidget` _widget)))
  (set `/Game/Blueprints/UI/PointsPopUp.ScoreValue` 1 _aspoints_pop_up))

(event `self.Sphere.OnComponentBeginOverlap`
  (params (OverlappedComponent :type "PrimitiveComponent Object Reference") (OtherActor :type "Actor Object Reference") (OtherComp :type "PrimitiveComponent Object Reference") (OtherBodyIndex :type Integer) (bFromSweep :type Boolean) (SweepResult :type "HitResult Structure (by ref)"))
  (bind (_returnvalue_x _returnvalue_y _returnvalue_z) (`KismetMathLibrary.BreakVector` (`self.K2_GetActorLocation`)))
  ;[1 1 1] Explosion
  (bind _asball_pawn (cast `/Game/Blueprints/Pawn/BallPawn` OtherActor))
  (`GameplayStatics.PlaySound2D` "/Game/StarterContent/Audio/Explosion01.Explosion01" 1.0 1.0 0.0 null null)
  (`GameplayStatics.SpawnEmitterAtLocation` "/Game/InfinityBladeEffects/Effects/FX_Monsters/FX_Monster_Gruntling/Bomber/P_FireBombExplosion.P_FireBombExplosion" (`KismetMathLibrary.MakeVector` _returnvalue_x _returnvalue_y _returnvalue_z) (struct) (5.0 5.0 5.0))
  (`PrimitiveComponent.AddRadialImpulse` (`/Game/Blueprints/Pawn/BallPawn.BallMesh` _asball_pawn) (`KismetMathLibrary.MakeVector` _returnvalue_x _returnvalue_y (- _returnvalue_z 50.0)) 500.0 1000.0 "RIF_Constant" true)
  (`self.K2_DestroyActor`))

(fn `UserConstructionScript`)