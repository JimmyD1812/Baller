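; BP_Star is a collectible star pickup that adds one point to a BP_BallPawn's score.
; When the pawn overlaps its sphere, it plays a coin sound and particles, hides the mesh and shows a points pop-up widget.
; A short delay keeps the pop-up visible before the actor destroys itself.
; Spin and Bounce timelines are set up to animate the mesh, but nothing in the graph starts them.
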(event `self.ReceiveBeginPlay`
  (bind _widget (`self.Widget`))
  (`SceneComponent.SetVisibility` _widget false false)
  (bind _asw_points_pop_up (cast `/Game/Blueprints/UI/W_PointsPopUp` (`WidgetComponent.GetWidget` _widget)))
  (set `/Game/Blueprints/UI/W_PointsPopUp.ScoreValue` 1 _asw_points_pop_up))

(event `self.Sphere.OnComponentBeginOverlap`
  (params (OverlappedComponent :type "PrimitiveComponent Object Reference") (OtherActor :type "Actor Object Reference") (OtherComp :type "PrimitiveComponent Object Reference") (OtherBodyIndex :type Integer) (bFromSweep :type Boolean) (SweepResult :type "HitResult Structure (by ref)"))
  ;[1 1 1] Increment Score
  (bind _asbp_ball_pawn (cast `/Game/Blueprints/Pawn/BP_BallPawn` OtherActor))
  (set `/Game/Blueprints/Pawn/BP_BallPawn.Score` (+ (`/Game/Blueprints/Pawn/BP_BallPawn.Score` _asbp_ball_pawn) 1) _asbp_ball_pawn)
  (`GameplayStatics.PlaySound2D` "/Game/Interface_And_Item_Sounds/WAV/Coins_08.Coins_08" 1.0 1.0 0.0 null null)
  (`GameplayStatics.SpawnEmitterAtLocation` (`self.OnPickupParticles`) (`self.K2_GetActorLocation`))
  (`SceneComponent.SetVisibility` (`self.StaticMesh`) false false)
  (`SceneComponent.SetVisibility` (`self.Widget`) true false)
  (`KismetSystemLibrary.Delay` 0.75)
  (`self.K2_DestroyActor`))

(fn `UserConstructionScript`)