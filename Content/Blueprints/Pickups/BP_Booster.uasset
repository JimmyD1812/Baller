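; BP_Booster is a boost pickup or pad that launches the player's ball when it overlaps the Booster component.
; On overlap with a BP_BallPawn, it applies an impulse to BallMesh as a velocity change, ignoring mass.
; The impulse is the offset from Arrow to Booster times BoostStrength, unnormalized, so component placement sets both direction and strength.
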(event `self.Booster.OnComponentBeginOverlap`
  (params (OverlappedComponent :type "PrimitiveComponent Object Reference") (OtherActor :type "Actor Object Reference") (OtherComp :type "PrimitiveComponent Object Reference") (OtherBodyIndex :type Integer) (bFromSweep :type Boolean) (SweepResult :type "HitResult Structure (by ref)"))
  (bind _boost_strength (`self.Boost Strength`))
  (bind (_returnvalue_x _returnvalue_y _returnvalue_z) (`KismetMathLibrary.BreakVector` (`SceneComponent.K2_GetComponentLocation` (`self.Arrow`))))
  (bind (_returnvalue_x_2 _returnvalue_y_2 _returnvalue_z_2) (`KismetMathLibrary.BreakVector` (`SceneComponent.K2_GetComponentLocation` (`self.Booster`))))
  (bind _asball_pawn (cast `/Game/Blueprints/Pawn/BP_BallPawn` OtherActor))
  (`PrimitiveComponent.AddImpulse` (`/Game/Blueprints/Pawn/BP_BallPawn.BallMesh` _asball_pawn) (`KismetMathLibrary.MakeVector` (* (- _returnvalue_x_2 _returnvalue_x) _boost_strength) (* (- _returnvalue_y_2 _returnvalue_y) _boost_strength) (* (- _returnvalue_z_2 _returnvalue_z) _boost_strength)) "None" true))

(fn `UserConstructionScript`)