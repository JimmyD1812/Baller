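; BP_Gear is a speed-boost pickup that temporarily raises the rolling ball pawn's torque and adds to its score.
; Overlapping its sphere plays sound and particles, hides the mesh, shows a points popup widget and destroys the trigger.
; After delays it removes the torque bonus and destroys itself; the popup stays visible until then.
; A Spin timeline meant to rotate the arrow is never started.
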(event `self.ReceiveBeginPlay`
  (bind _widget (`self.Widget`))
  (`SceneComponent.SetVisibility` _widget false false)
  (bind _aspoints_pop_up (cast `/Game/Blueprints/UI/W_PointsPopUp` (`WidgetComponent.GetWidget` _widget)))
  (set `/Game/Blueprints/UI/W_PointsPopUp.ScoreValue` 5 _aspoints_pop_up))

(event `self.Sphere.OnComponentBeginOverlap`
  (params (OverlappedComponent :type "PrimitiveComponent Object Reference") (OtherActor :type "Actor Object Reference") (OtherComp :type "PrimitiveComponent Object Reference") (OtherBodyIndex :type Integer) (bFromSweep :type Boolean) (SweepResult :type "HitResult Structure (by ref)"))
  ;[1 1 1] Go Fast
  (bind _asbp_ball_pawn (cast `/Game/Blueprints/Pawn/BP_BallPawn` OtherActor))
  (set `/Game/Blueprints/Pawn/BP_BallPawn.Torque` (+ (`/Game/Blueprints/Pawn/BP_BallPawn.Torque` _asbp_ball_pawn) 2000.0) _asbp_ball_pawn)
  (set `/Game/Blueprints/Pawn/BP_BallPawn.Score` (+ (`/Game/Blueprints/Pawn/BP_BallPawn.Score` _asbp_ball_pawn) 5) _asbp_ball_pawn)
  (`GameplayStatics.PlaySound2D` "/Game/Interface_And_Item_Sounds/Cues/Pop_06_Cue.Pop_06_Cue" 1.0 1.0 0.0 null null)
  (`GameplayStatics.SpawnEmitterAtLocation` (`self.On Pickup Particles`) (`self.K2_GetActorLocation`))
  (`SceneComponent.SetVisibility` (`self.StaticMesh`) false false)
  (`SceneComponent.SetVisibility` (`self.Widget`) true false)
  (`ActorComponent.K2_DestroyComponent` (`self.Sphere`))
  (`KismetSystemLibrary.Delay` 0.75)
  (`SceneComponent.SetVisibility` (`self.Widget`) true false)
  (`KismetSystemLibrary.Delay` 15.0)
  (set `/Game/Blueprints/Pawn/BP_BallPawn.Torque` (- (`/Game/Blueprints/Pawn/BP_BallPawn.Torque` _asbp_ball_pawn) 2000.0) _asbp_ball_pawn)
  (`self.K2_DestroyActor`))

(fn `UserConstructionScript`)